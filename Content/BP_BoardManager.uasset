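; Board manager for a grid-based card unit game, spawning a small grid of BP_Tile actors on BeginPlay and storing their coordinates.
; It highlights move range by Manhattan distance and Forward attack tiles in the unit's column, though that check never compares tile GridY.
; ReserveMove validates targets against DT_CardList MoveRange and stores one reservation per player.
; ExecuteTurn is empty, and the GridToWorld and GetTileAt returns are unwired.
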(event `self.ReceiveBeginPlay`
  (for _index (range 3)
    (for _index_2 (range 7)
      (bind _returnvalue (`|SpawnActorFromClass` "/Game/BP_Tile.BP_Tile_C" (`KismetMathLibrary.MakeTransform` (`KismetMathLibrary.MakeVector` (`KismetMathLibrary.Conv_IntToDouble` (* _index 100)) (`KismetMathLibrary.Conv_IntToDouble` (* _index_2 100)))) "Undefined" "MultiplyWithRoot" null null))
      (set `/Game/BP_Tile.GridX` _index _returnvalue)
      (set `/Game/BP_Tile.GridY` _index_2 _returnvalue)
      (`KismetArrayLibrary.Array_Add` (`self.Tiles`) _returnvalue))))

(fn `ExecuteTurn`)

(fn `GetTileAt`
  (params (GridX :type Integer) (GridY :type Integer))
  (returns (FoundTile :type "/Game/BP_Tile Object Reference"))
  (for _array_element (`self.Tiles`)
    _))

(fn `GridToWorld`
  (params (GridX :type Integer) (GridY :type Integer))
  (returns (WorldLocation :type "Vector Structure")))

(fn `ReserveMove`
  (params (UnitReference :type "/Game/BP_Unit Object Reference") (NewGridX :type Integer) (NewGridY :type Integer))
  (`KismetSystemLibrary.PrintString` "ReserveMoveCalled")
  (bind _returnvalue (`|GetDataTableRow` "/Game/DT_CardList.DT_CardList" (`/Game/BP_Unit.RowName` UnitReference))
    (:`then`
      (if (<= (+ (`KismetMathLibrary.Abs_Int` (- (`/Game/BP_Unit.GridX` UnitReference) NewGridX)) (`KismetMathLibrary.Abs_Int` (- (`/Game/BP_Unit.GridY` UnitReference) NewGridY))) (`.MoveRange_14_2C78F8CE4E77427D700B0884E05F0F5C` (break `/Game/S_CardData` _returnvalue)))
        (if (== (`/Game/BP_Unit.PlayerSide` UnitReference) 1)
          (set `self.P1_TargetGridX` NewGridX)
          (set `self.P1_TargetGridY` NewGridY)
          (set `self.P1HasReserved` true)
          (`KismetSystemLibrary.PrintString` "SetP1Reserved")
          (else
            (set `self.P2_TargetGridX` NewGridX)
            (set `self.P2_TargetGridY` NewGridY)
            (set `self.P2HasReserved` true)))))))

(fn `ResetAllTlies`
  (for _array_element (`self.Tiles`)
    (bind _asbp_tile (cast `/Game/BP_Tile` _array_element))
    (`/Game/BP_Tile.ResetTile` _asbp_tile)))

(fn `ShowAtackableTiles`
  (params (SelectedUnit :type "/Game/BP_Unit Object Reference") (Range :type Integer) (Pattern :type "/Game/EAtackPattern Enum" :default "NewEnumerator0"))
  (bind _gridy (`/Game/BP_Unit.GridY` SelectedUnit))
  (for _array_element (`self.Tiles`)
    (bind _asbp_tile (cast `/Game/BP_Tile` _array_element))
    (switch `/Game/EAtackPattern` Pattern
      (:`NewEnumerator1`
        (if (== (`/Game/BP_Unit.OwnerPlayer` SelectedUnit) 1)
          (bind _returnvalue (== (`/Game/BP_Tile.GridX` _asbp_tile) (`/Game/BP_Unit.GridX` SelectedUnit)))
          (if (and _returnvalue (`KismetMathLibrary.Conv_IntToBool` (- _gridy 1)))
            (`/Game/BP_Tile.ShowAtackRange` _asbp_tile))
          (elif (and _returnvalue (`KismetMathLibrary.Conv_IntToBool` (+ _gridy 1)))
            (`/Game/BP_Tile.ShowAtackRange` _asbp_tile)))))))

(fn `ShowMovableRange`
  (params (SelectedUnit :type "/Game/BP_Unit Object Reference") (Range :type Integer))
  (for _array_element (`self.Tiles`)
    (bind _asbp_tile (cast `/Game/BP_Tile` _array_element))
    (if (<= (+ (`KismetMathLibrary.Abs_Int` (- (`/Game/BP_Tile.GridX` _asbp_tile) (`/Game/BP_Unit.GridX` SelectedUnit))) (`KismetMathLibrary.Abs_Int` (- (`/Game/BP_Tile.GridY` _asbp_tile) (`/Game/BP_Unit.GridY` SelectedUnit)))) Range)
      (`/Game/BP_Tile.ShowMoveRange` _asbp_tile))))

(fn `UserConstructionScript`)