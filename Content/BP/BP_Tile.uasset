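; BP_Tile is a clickable grid board tile that holds its X/Y coordinate and shows range highlights.
; On click it asks the first UnitSpawn actor to spawn a unit at its grid position, scaled by 100 into world space.
; Move and attack range functions both apply the same highlight material, and ResetTile restores the normal one.
; Coordinate text, phase-based summon and move reservation, and an older spawn path are disconnected and never run.
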(event `self.ReceiveActorOnClicked`
  (params (ButtonPressed :type "Key Structure"))
  (bind _gridx (`self.GridX`))
  (bind _gridy (`self.GridY`))
  (bind _outactors (`GameplayStatics.GetAllActorsOfClass` "/Script/Rayla_Feat.UnitSpawn"))
  (`UnitSpawn.SpawnMyUnit` (`|GetArrayItem` _outactors) (`KismetMathLibrary.MakeVector` (* (`KismetMathLibrary.Conv_IntToDouble` _gridx) 100.0) (* (`KismetMathLibrary.Conv_IntToDouble` _gridy) 100.0)) (make `IntPoint` _gridx _gridy)))

(fn `ResetTile`
  (`PrimitiveComponent.SetMaterial` (`self.TileMesh`) 0 (`self.NormalMaterial`)))

(fn `ShowAtackRange`
  (`KismetSystemLibrary.PrintString` "攻撃可能範囲を今から見せるね")
  (`PrimitiveComponent.SetMaterial` (`self.TileMesh`) 0 (`self.HighLightMaterial`)))

(fn `ShowMoveRange`
  (`PrimitiveComponent.SetMaterial` (`self.TileMesh`) 0 (`self.HighLightMaterial`)))

(fn `UserConstructionScript`)