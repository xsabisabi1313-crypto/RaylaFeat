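; BP_Unit is a card-driven board unit that can be selected and moved on a tile grid, with stats loaded from DT_CardList by row name.
; In one GameMode phase, clicking toggles selection, registering it with BP_GameMode and showing its movable range through BP_BoardManager.
; In another phase, ExecuteMove teleports it to the tile, flags a base (kyoten) attack at row Y=0, and highlights its computed attack range.
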(event `self.ReceiveActorOnClicked`
  (params (ButtonPressed :type "Key Structure"))
  (bind _asbp_game_mode (cast `/Game/BP/BP_GameMode` (`GameplayStatics.GetGameMode`)))
  (if (`|EnumEquality` (`/Game/BP/BP_GameMode.CurrentPhase` _asbp_game_mode) "NewEnumerator1")
    (set `self.IsSelected` (not (`self.IsSelected`)))
    (if (`self.IsSelected`)
      (`self.SelectUnit`)
      (`KismetSystemLibrary.PrintString` "選んだ" false)
      (bind _returnvalue (`GameplayStatics.GetActorOfClass` "/Game/BP/BP_BoardManager.BP_BoardManager_C"))
      (`/Game/BP/BP_BoardManager.ShowMovableRange` _returnvalue self (`self.MoveRange`))
      (cast `/Game/BP/BP_GameMode` (`GameplayStatics.GetGameMode`))
      (`self.SelectUnit`)
      (else
        (`KismetSystemLibrary.PrintString` "選択解除" false)))))

(fn `ExecuteMove`
  (params (NewTargetGridX :type Integer) (NewTargetGridY :type Integer))
  (bind _asbp_game_mode (cast `/Game/BP/BP_GameMode` (`GameplayStatics.GetGameMode`)))
  (if (`|EnumEquality` (`/Game/BP/BP_GameMode.CurrentPhase` _asbp_game_mode) "NewEnumerator5")
    (`self.MoveToGrid` NewTargetGridX NewTargetGridY)))

(fn `InitializeCardData`
  (bind _rowname (`self.RowName`))
  (`KismetSystemLibrary.PrintString` (`KismetStringLibrary.Conv_NameToString` _rowname) false)
  (bind _returnvalue (`|GetDataTableRow` "/Game/Data/DT_CardList.DT_CardList" _rowname)
    (:`then`
      (bind ((`Cost_7_B5082ECF41B755D5A640ACAD3DE0068E` _cost) (`Power_9_8C7743F842BA5A693FD46B9223594953` _power) (`Element_11_9FD03F7B46E01A1EC38D4A989718CFE1` _element) (`MoveRange_14_2C78F8CE4E77427D700B0884E05F0F5C` _moverange) (`AtackRange_16_74110C0248143538DA3BEFBB34E251BF` _atackrange) (`AtackPattern_23_3CF1077646172493D0D54DAB54A8EF97` _atackpattern)) (break `/Game/Data/S_CardData` _returnvalue))
      (set `self.Cost` _cost)
      (bind _output_get (set `self.Power` _power))
      (`KismetSystemLibrary.PrintString` (`KismetStringLibrary.Conv_IntToString` _output_get) false)
      (set `self.Element` _element)
      (set `self.MoveRange` _moverange)
      (set `self.AtackRange` _atackrange)
      (set `self.AtackPattern` _atackpattern))))

(fn `MoveToGrid`
  (params (NewGridX :type Integer) (NewGridY :type Integer))
  (`GameplayStatics.PlaySoundAtLocation` "/Game/Sound/構えを取る__1_.構えを取る__1_" (0.0 0.0 0.0) (struct) 1.0 1.0 0.0 null null null null)
  (bind _asbp_game_mode (cast `/Game/BP/BP_GameMode` (`GameplayStatics.GetGameMode`)))
  (set `/Game/BP/BP_GameMode.isAttackKyoten` (== NewGridY 0) _asbp_game_mode)
  (bind _output_get (set `self.GridX` NewGridX))
  (bind _output_get_2 (set `self.GridY` NewGridY))
  (bind _returnvalue (`|GetDataTableRow` "/Game/Data/DT_CardList.DT_CardList" (`self.RowName`))
    (:`then`
      (bind _returnvalue_2 (`self.CalculateAttackRange` _output_get _output_get_2 (`self.PlayerSide`) (`.AtackPattern_23_3CF1077646172493D0D54DAB54A8EF97` (break `/Game/Data/S_CardData` _returnvalue)) (`.AtackRange_16_74110C0248143538DA3BEFBB34E251BF` (break `/Game/Data/S_CardData` _returnvalue))))
      (set `self.AttackRangePriority` _returnvalue_2)
      (`self.ShowAttackRangeFromArray`)
      (bind _returnvalue_3 (`GameplayStatics.GetActorOfClass` "/Game/BP/BP_BoardManager.BP_BoardManager_C"))
      (`self.K2_SetActorLocation` (`self.K2_GetActorLocation` (`|GetArrayItem` (`/Game/BP/BP_BoardManager.Tiles` _returnvalue_3) (+ (* (`local.NewGridX`) 7) (`local.NewGridY`))))))))

(fn `SelectUnit`
  (`KismetSystemLibrary.PrintString` "Hello")
  (bind _asbp_game_mode (cast `/Game/BP/BP_GameMode` (`GameplayStatics.GetGameMode`)))
  (`/Game/BP/BP_GameMode.SetSelectedUnit` _asbp_game_mode self))

(fn `ShowAttackRangeFromArray`
  (`GameplayStatics.GetActorOfClass` "/Game/BP/BP_Tile.BP_Tile_C")
  (for _array_element _
    (bind _asbp_tile (cast `/Game/BP/BP_Tile` _array_element))
    (for _array_element_2 (`self.AttackRangePriority`)
      (bind (_x _y) (break `IntPoint` _array_element_2))
      (if (and (== _x (`/Game/BP/BP_Tile.GridX` _asbp_tile)) (== _y (`/Game/BP/BP_Tile.GridY` _asbp_tile)))
        (`/Game/BP/BP_Tile.ShowAtackRange` _asbp_tile)))))

(fn `UserConstructionScript`)