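; Game mode for a grid-based card battler, running Spawn, Move Reserve, Battle and an empty Game Over phase through ChangePhase.
; Spawn shows cost and confirm widgets, SummonUnit places units against Player2Cost for both sides, and DebugSpawnEnemy drops scripted enemies on random tiles.
; Move Reserve executes moves stored in BP_BoardManager.
; Battle resolves pairs using power and a Fire/Water/Grass check, destroying units and reducing HP on target actors.
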(event `self.ReceiveBeginPlay`
  (`self.StartCardPhase`)
  (bind _asbp_game_mode (cast `/Game/BP/BP_GameMode` (`GameplayStatics.GetGameMode`)))
  (set `/Game/BP/BP_GameMode.CurrentPhase` "NewEnumerator0" _asbp_game_mode)
  (bind _asbp_game_mode_2 (cast `/Game/BP/BP_GameMode` (`GameplayStatics.GetGameMode`)))
  (`self.DebugSpawnEnemy` _asbp_game_mode_2))

(fn `BattleUnits`
  (params (Unit1Power :type Integer) (Unit1Element :type "/Game/Data/E_Element Enum" :default "NewEnumerator0") (Unit2Power :type Integer) (Unit2Element :type "/Game/Data/E_Element Enum" :default "NewEnumerator0"))
  (returns (Result :type String))
  (locals (Final_Unit1_Power :type Integer) (Final_Unit2_Power :type Integer))
  (bind _final_unit1_power (`local.Final_Unit1_Power`))
  (bind _final_unit2_power (`local.Final_Unit2_Power`))
  (bind _isadvantage (`self.CheckElementAdvantage` Unit1Element Unit2Element))
  (if _isadvantage
    (set `local.Final_Unit1_Power` (* Unit1Power 2))
    (else
      (set `local.Final_Unit2_Power` Unit2Power)))
  (bind _isadvantage_2 (`self.CheckElementAdvantage` Unit1Element Unit2Element))
  (if _isadvantage_2
    (set `local.Final_Unit2_Power` (* Unit2Power 2))
    (else
      (set `local.Final_Unit2_Power` Unit2Power)))
  (if (< _final_unit1_power _final_unit2_power)
    (return "Unit1の勝利")
    (elif (> _final_unit1_power _final_unit2_power)
      (return "Unit2の勝利")
      (else
        (return "相打ち")))))

(fn `ChangePhase`
  (params (NewPhase :type "/Game/Data/EGamePhase Enum" :default "NewEnumerator0"))
  (`KismetSystemLibrary.PrintString` (`|GetEnumeratorNameAsString` NewPhase) false true (struct :`A` 1.0))
  (set `self.CurrentPhase` NewPhase)
  (`KismetSystemLibrary.PrintString` (`KismetStringLibrary.Conv_IntToString` (`self.TurnCount`)) false true (struct :`R` 0.018224 :`G` 0.923333 :`A` 1.0) 10.0)
  (`self.OnPhaseChanged` NewPhase)
  (switch `/Game/Data/EGamePhase` NewPhase
    (:`NewEnumerator0`
      (bind _returnvalue (`GameplayStatics.GetActorOfClass` "/Game/BP/BP_BoardManager.BP_BoardManager_C"))
      (set `/Game/BP/BP_BoardManager.P1HasReserved` false _returnvalue)
      (set `/Game/BP/BP_BoardManager.P2HasReserved` false _returnvalue)
      (`self.StartCardPhase`))
    (:`NewEnumerator1`
      (`self.StartProcess`))
    (:`NewEnumerator2`
      (`self.StartBattle`))
    (:`NewEnumerator3`
      (`self.StartGameOver`))))

(fn `CheckElementAdvantage`
  (params (AtackerElement :type "/Game/Data/E_Element Enum" :default "NewEnumerator0") (DefenderElement :type "/Game/Data/E_Element Enum" :default "NewEnumerator0"))
  (returns (IsAdvantage :type Boolean))
  (switch `/Game/Data/E_Element` AtackerElement
    (:`NewEnumerator0`
      (return (`|EnumEquality` DefenderElement "NewEnumerator2")))
    (:`NewEnumerator1`
      (return (`|EnumEquality` DefenderElement "NewEnumerator0")))
    (:`NewEnumerator2`
      (return (`|EnumEquality` DefenderElement "NewEnumerator1")))))

(fn `DebugSpawnEnemy`
  (bind _returnvalue (`GameplayStatics.GetActorOfClass` "/Game/BP/BP_BoardManager.BP_BoardManager_C"))
  (bind _output_get (set `self.PosXtemp` (`KismetMathLibrary.RandomIntegerInRange` 0 2)))
  (bind _output_get_2 (set `self.PosYtemp` (`KismetMathLibrary.RandomIntegerInRange` 0 2)))
  (bind _foundtile (`/Game/BP/BP_BoardManager.GetTileAt` _returnvalue _output_get _output_get_2))
  (switch `int` (`self.enemyspawnindex`)
    (:`Default`
      (`KismetSystemLibrary.PrintString` "Hello" false))
    (:`0`
      (bind _returnvalue_2 (`KismetSystemLibrary.IsValid` _foundtile))
      (if _returnvalue_2
        (bind _returnvalue_3 (`self.GetTransform` _foundtile))
        (bind _returnvalue_4 (`|SpawnActorFromClass` "/Game/BP/BP_Unit_RedRidingHood.BP_Unit_RedRidingHood_C" _returnvalue_3 "Undefined" "MultiplyWithRoot" null null))
        (if (`KismetSystemLibrary.IsValid` _returnvalue_4)
          (`/Game/BP/BP_Unit.InitializeCardData` _returnvalue_4)
          (bind _asbp_unit (cast `/Game/BP/BP_Unit` _returnvalue_4))
          (if (`KismetSystemLibrary.IsValid` _asbp_unit)
            (set `/Game/BP/BP_Unit.RowName` "RedRidingHood" _asbp_unit)
            (set `BP_UnitBase.GridX` (`self.PosXtemp`) _asbp_unit)
            (set `BP_UnitBase.GridY` (`self.PosYtemp`) _asbp_unit)
            (bind _result (`/Engine/EditorBlueprintResources/StandardMacros.IncrementInt` (`self.enemyspawnindex`) :!label _label)
              (:`  `
                (set `self.enemyspawnindex` _result)
                (`GameplayStatics.PlaySound2D` "/Game/Sound/選択4.選択4" 1.0 1.0 0.0 null null)
                (bind _returnvalue_5 (`GameplayStatics.GetActorOfClass` "/Game/BP/BP_BoardManager.BP_BoardManager_C"))
                (set `/Game/BP/BP_BoardManager.P2_SelectedUnit` null _returnvalue_5)))))))
    (:`1`
      (if _returnvalue_2
        (bind _returnvalue_6 (`|SpawnActorFromClass` "/Game/BP/BP_Unit_ryouju.BP_Unit_ryouju_C" _returnvalue_3 "Undefined" "MultiplyWithRoot" null null))
        (if (`KismetSystemLibrary.IsValid` _returnvalue_6)
          (`/Game/BP/BP_Unit.InitializeCardData` _returnvalue_6)
          (bind _asbp_unit_2 (cast `/Game/BP/BP_Unit` _returnvalue_6))
          (if (`KismetSystemLibrary.IsValid` _asbp_unit_2)
            (set `/Game/BP/BP_Unit.RowName` "Ryoju" _asbp_unit_2)
            (set `BP_UnitBase.GridY` (`self.PosYtemp`) _asbp_unit_2)
            (set `BP_UnitBase.GridX` (`self.PosXtemp`) _asbp_unit_2)
            (goto _label)))))
    (:`2`
      (if _returnvalue_2
        (bind _returnvalue_7 (`|SpawnActorFromClass` "/Game/BP/BP_Unit_grandmother.BP_Unit_grandmother_C" _returnvalue_3 "Undefined" "MultiplyWithRoot" null null))
        (if (`KismetSystemLibrary.IsValid` _returnvalue_7)
          (`/Game/BP/BP_Unit.InitializeCardData` _returnvalue_7)
          (bind _asbp_unit_3 (cast `/Game/BP/BP_Unit` _returnvalue_7))
          (if (`KismetSystemLibrary.IsValid` _asbp_unit_3)
            (set `/Game/BP/BP_Unit.RowName` "Granma" _asbp_unit_3)
            (set `BP_UnitBase.GridY` (`self.PosYtemp`) _asbp_unit_3)
            (set `BP_UnitBase.GridX` (`self.PosXtemp`) _asbp_unit_3)
            (goto _label)))))))

(fn `MoveEnemy`
  (bind _returnvalue (`GameplayStatics.GetActorOfClass` "/Game/BP/BP_BoardManager.BP_BoardManager_C"))
  (bind _p2_selectedunit (`/Game/BP/BP_BoardManager.P2_SelectedUnit` _returnvalue))
  (`/Engine/EditorBlueprintResources/StandardMacros.IsValid` _p2_selectedunit
    (:`Is Valid`
      (if (`/Game/BP/BP_BoardManager.P2HasReserved` _returnvalue)
        (`/Game/BP/BP_Unit.ExecuteMove` _p2_selectedunit (`/Game/BP/BP_BoardManager.P2_TargetGridX` _returnvalue) (`/Game/BP/BP_BoardManager.P2_TargetGridY` _returnvalue))))))

(fn `PlayerConfirm`
  (params (PlayerID :type Integer))
  (if (== PlayerID 1)
    (set `self.Player1Confirmed` true)))

(fn `SetSelectedUnit`
  (params (UnitReference :type "/Game/BP/BP_Unit Object Reference"))
  (bind _returnvalue (`GameplayStatics.GetActorOfClass` "/Game/BP/BP_BoardManager.BP_BoardManager_C"))
  (set `/Game/BP/BP_BoardManager.P1_SelectedUnit` UnitReference _returnvalue)
  (`KismetSystemLibrary.PrintString` "UNITSTORED" false))

(fn `StartBattle`
  (locals (P1MovedUnit :type "/Game/BP/BP_Unit Object Reference") (P2MovedUnit :type "/Game/BP/BP_Unit Object Reference"))
  (bind _hpactor (`/Game/BP/Kyoten.HPActor` (`self.TargetAC1`)))
  (bind _hpactor_2 (`/Game/BP/Kyoten.HPActor` (`self.TargetAC2`)))
  (bind _hpactor_3 (`/Game/BP/Kyoten.HPActor` (`self.TargetAC2`)))
  (if (`self.isAttackKyoten`)
    (bind _foundwidgets (`WidgetBlueprintLibrary.GetAllWidgetsOfClass` "/Game/WBP/WB_ConfirmButton.WB_ConfirmButton_C"))
    (`HPActorComponent.ReduceHP` _hpactor_2 5.0)
    (`/Game/WBP/WB_ConfirmButton.changeEnemyHPText` (`|GetArrayItem` _foundwidgets) (`KismetStringLibrary.Conv_Int64ToString` (`KismetMathLibrary.Conv_DoubleToInt64` (`HPActorComponent.Health` _hpactor_2))))
    (set `self.isAttackKyoten` false))
  (`KismetSystemLibrary.PrintString` "バトルフェーズ開始" true true (struct :`R` 0.723333 :`G` 0.214145 :`A` 1.0))
  (bind _returnvalue (`GameplayStatics.GetActorOfClass` "/Game/BP/BP_BoardManager.BP_BoardManager_C"))
  (if (`/Game/BP/BP_BoardManager.P1HasReserved` _returnvalue)
    (set `local.P1MovedUnit` (`/Game/BP/BP_BoardManager.P1_SelectedUnit` _returnvalue)))
  (if (`/Game/BP/BP_BoardManager.P2HasReserved` _returnvalue)
    (set `local.P2MovedUnit` (`/Game/BP/BP_BoardManager.P2_SelectedUnit` _returnvalue)))
  (bind _outactors (`GameplayStatics.GetAllActorsOfClass` "/Game/BP/BP_Unit.BP_Unit_C"))
  (bind _returnvalue_2 (`self.DetermineBattlePairs` (`local.P1MovedUnit`) (`local.P2MovedUnit`) _outactors))
  (for _array_element _returnvalue_2
    (bind _asbp_unit (cast `/Game/BP/BP_Unit` (break `BattlePair` _array_element)))
    (bind _asbp_unit_2 (cast `/Game/BP/BP_Unit` (`.UnitB` (break `BattlePair` _array_element))))
    (bind _result (`self.BattleUnits` (`/Game/BP/BP_Unit.Power` _asbp_unit) (`/Game/BP/BP_Unit.Element` _asbp_unit) (`/Game/BP/BP_Unit.Power` _asbp_unit_2) (`/Game/BP/BP_Unit.Element` _asbp_unit_2)))
    (bind _foundwidgets_2 (`WidgetBlueprintLibrary.GetAllWidgetsOfClass` "/Game/WBP/WB_ConfirmButton.WB_ConfirmButton_C"))
    (`GameplayStatics.PlaySoundAtLocation` "/Game/Sound/鞭で攻撃.鞭で攻撃" (0.0 0.0 0.0) (struct) 1.0 1.0 0.0 null null null null)
    (switch `string` _result
      (:`Unit1の勝利`
        (`self.K2_DestroyActor` (`.UnitB` (break `BattlePair` _array_element)))
        (`KismetSystemLibrary.PrintString` "Unit1の勝利" false)
        (`HPActorComponent.ReduceHP` _hpactor 5.0)
        (bind _output (`|GetArrayItem` _foundwidgets_2))
        (`/Game/WBP/WB_ConfirmButton.changeFriendHPText` _output (`KismetStringLibrary.Conv_Int64ToString` (`KismetMathLibrary.Conv_DoubleToInt64` (`HPActorComponent.Health` _hpactor)))))
      (:`Unit2の勝利`
        (`self.K2_DestroyActor` (break `BattlePair` _array_element))
        (`KismetSystemLibrary.PrintString` "Unit2の勝利" false)
        (`HPActorComponent.ReduceHP` _hpactor_3 5.0)
        (`/Game/WBP/WB_ConfirmButton.changeEnemyHPText` _output (`KismetStringLibrary.Conv_Int64ToString` (`KismetMathLibrary.Conv_DoubleToInt64` (`HPActorComponent.Health` _hpactor_3)))))
      (:`相打ち`
        (`self.K2_DestroyActor` (break `BattlePair` _array_element))
        (`self.K2_DestroyActor` (`.UnitB` (break `BattlePair` _array_element)))
        (`KismetSystemLibrary.PrintString` "相打ち" false)))
    (`KismetSystemLibrary.PrintString` "Battleフェーズ終了で！！" false true (struct :`R` 0.776667 :`G` 0.43432 :`A` 1.0) 10.0)))

(fn `StartCardPhase`
  (bind _returnvalue (`GameplayStatics.GetPlayerController` 0))
  (bind _returnvalue_2 (`GameplayStatics.GetPlayerController` 0))
  (if (not (== (`self.TurnCount`) 1))
    (set `self.Player1Cost` (+ (`self.Player1Cost`) 2))
    (set `self.Player2Cost` (+ (`self.Player2Cost`) 2)))
  (bind _returnvalue_3 (`|CreateWidget` "/Game/WBP/WB_ConfirmButton.WB_ConfirmButton_C" _returnvalue))
  (`UserWidget.AddToViewport` _returnvalue_3 0)
  (bind _returnvalue_4 (`|CreateWidget` "/Game/WBP/WB_CostDisplay.WB_CostDisplay_C" _returnvalue))
  (bind _output_get (set `self.CostDisplayWidget` _returnvalue_4))
  (`UserWidget.AddToViewport` _output_get 0)
  (`/Game/WBP/WB_CostDisplay.UpdateCostDisplay` _output_get (`self.Player1Cost`) (`self.Player2Cost`))
  (`KismetSystemLibrary.PrintString` "ここから先を調整しようと思います" false false)
  (`WidgetBlueprintLibrary.SetInputMode_GameAndUIEx` _returnvalue_2 (stale _aswb_confirm_button))
  (bind _aswb_confirm_button (cast `/Game/WBP/WB_ConfirmButton` _returnvalue_3))
  (bind _output_get_2 (set `PlayerController.bShowMouseCursor` true _returnvalue_2))
  (set `PlayerController.bEnableClickEvents` _output_get_2 _returnvalue_2))

(fn `StartGameOver`)

(fn `StartProcess`
  (`self.MoveEnemy`)
  (bind _returnvalue (`GameplayStatics.GetActorOfClass` "/Game/BP/BP_BoardManager.BP_BoardManager_C"))
  (bind _p1_selectedunit (`/Game/BP/BP_BoardManager.P1_SelectedUnit` _returnvalue))
  (`/Engine/EditorBlueprintResources/StandardMacros.IsValid` _p1_selectedunit
    (:`Is Valid`
      (if (`/Game/BP/BP_BoardManager.P1HasReserved` _returnvalue)
        (`/Game/BP/BP_Unit.ExecuteMove` _p1_selectedunit (`/Game/BP/BP_BoardManager.P1_TargetGridX` _returnvalue) (`/Game/BP/BP_BoardManager.P1_TargetGridY` _returnvalue))))))

(fn `SummonUnit`
  (params (SpawnTile :type "/Game/BP/BP_Tile Object Reference") (UnitClass :type "/Game/BP/BP_Unit Class Reference") (PlayerID :type Integer) (RowName :type Name))
  (bind _returnvalue (`self.GetTransform` SpawnTile))
  (bind (_isselected _targetgridx _targetgridy _power _element _rowname _ownerplayer _moverange _atackrange _atackpattern _cost) (defaults `Object` UnitClass))
  (if (== PlayerID 1)
    (if (>= (`self.Player2Cost`) _cost)
      (`GameplayStatics.PlaySoundAtLocation` "/Game/Sound/選択4.選択4" (0.0 0.0 0.0) (struct) 1.0 1.0 0.0 null null null null)
      (bind _returnvalue_2 (`|SpawnActorFromClass` UnitClass _returnvalue "Undefined" "MultiplyWithRoot" null null))
      (set `/Game/BP/BP_Unit.OwnerPlayer` 1 _returnvalue_2)
      (set `/Game/BP/BP_Unit.GridX` (`/Game/BP/BP_Tile.GridX` SpawnTile) _returnvalue_2)
      (set `/Game/BP/BP_Unit.GridY` (`/Game/BP/BP_Tile.GridY` SpawnTile) _returnvalue_2)
      (bind _output_get (set `self.Player2Cost` (- (`self.Player2Cost`) (`/Game/BP/BP_Unit.Cost` _returnvalue_2))))
      (set `self.UnitToSummon` null)
      (set `/Game/BP/BP_Unit.RowName` RowName _returnvalue_2)
      (`/Game/BP/BP_Unit.InitializeCardData` _returnvalue_2)
      (`KismetSystemLibrary.PrintString` "味方スポーン!" false)
      (`self.K2_AddActorWorldRotation` _returnvalue_2 (struct :`Yaw` 180.0) false false)
      (bind _foundwidgets (`WidgetBlueprintLibrary.GetAllWidgetsOfClass` "/Game/WBP/WB_CostDisplay.WB_CostDisplay_C"))
      (bind _aswb_cost_display (cast `/Game/WBP/WB_CostDisplay` (`|GetArrayItem` _foundwidgets)))
      (`/Game/WBP/WB_CostDisplay.UpdateCostDisplay` _aswb_cost_display 0 _output_get)
      (else
        (`KismetSystemLibrary.PrintString` "コストが足りません！" true true (struct :`R` 0.567333 :`A` 1.0))))
    (elif (>= (`self.Player2Cost`) _cost)
      (bind _returnvalue_3 (`|SpawnActorFromClass` UnitClass _returnvalue "Undefined" "MultiplyWithRoot" null null))
      (set `/Game/BP/BP_Unit.OwnerPlayer` 2 _returnvalue_3)
      (set `/Game/BP/BP_Unit.GridX` (`/Game/BP/BP_Tile.GridX` SpawnTile) _returnvalue_3)
      (set `/Game/BP/BP_Unit.GridY` (`/Game/BP/BP_Tile.GridY` SpawnTile) _returnvalue_3)
      (set `self.Player2Cost` (- (`self.Player2Cost`) (`/Game/BP/BP_Unit.Cost` _returnvalue_3)))
      (set `self.UnitToSummon` null))))

(fn `UserConstructionScript`)