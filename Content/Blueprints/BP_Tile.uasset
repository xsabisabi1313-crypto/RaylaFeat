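; BP_Tile is a clickable grid tile that sends the selected unit to its coordinates.
; On click, it finds BP_BoardManager and, if a SelectedUnit is valid, copies its GridX and GridY into the unit's target.
; It then prints a debug message and calls ExecuteMove on that unit immediately.
; Logic to show the coordinates on CoordinateText exists but is unconnected, so it never runs.
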(event `self.ReceiveActorOnClicked`
  (params (ButtonPressed :type "Key Structure"))
  (bind _returnvalue (`GameplayStatics.GetActorOfClass` "/Game/Blueprints/BP_BoardManager.BP_BoardManager_C"))
  (bind _selectedunit (`/Game/Blueprints/BP_BoardManager.SelectedUnit` _returnvalue))
  (`/Engine/EditorBlueprintResources/StandardMacros.IsValid` _selectedunit
    (:`Is Valid`
      (set `/Game/Blueprints/BP_Unit.TargetGridX` (`self.GridX`) _selectedunit)
      (set `/Game/Blueprints/BP_Unit.TargetGridY` (`self.GridY`) _selectedunit)
      (`KismetSystemLibrary.PrintString` "MOVE RESERBED")
      (`/Game/Blueprints/BP_Unit.ExecuteMove` _selectedunit))))

(fn `UserConstructionScript`)