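; Board manager that builds the grid for a tile-based unit game when play begins.
; Nested loops spawn a 3x7 field of BP_Tile actors at fixed spacing, give each its grid coordinates and store them in Tiles, then place one BP_Unit on the first tile.
; GridToWorld, GetTileAt and ExecuteTurn are unfinished, with empty or disconnected logic, and the unit move and selection test nodes are unwired.
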(event `self.ReceiveBeginPlay`
  (for _index (range 3)
    (for _index_2 (range 7)
      (bind _returnvalue (`|SpawnActorFromClass` "/Game/Blueprints/BP_Tile.BP_Tile_C" (`KismetMathLibrary.MakeTransform` (`KismetMathLibrary.MakeVector` (`KismetMathLibrary.Conv_IntToDouble` (* _index 100)) (`KismetMathLibrary.Conv_IntToDouble` (* _index_2 100)))) "Undefined" "MultiplyWithRoot" null null))
      (set `/Game/Blueprints/BP_Tile.GridX` _index _returnvalue)
      (set `/Game/Blueprints/BP_Tile.GridY` _index_2 _returnvalue)
      (`KismetArrayLibrary.Array_Add` (`self.Tiles`) _returnvalue)))
  (bind _returnvalue_2 (`|SpawnActorFromClass` "/Game/Blueprints/BP_Unit.BP_Unit_C" (`KismetMathLibrary.MakeTransform` (`self.K2_GetActorLocation` (`|GetArrayItem` (`self.Tiles`)))) "Undefined" "MultiplyWithRoot" null null)))

(fn `ExecuteTurn`)

(fn `GetTileAt`
  (params (GridX :type Integer) (GridY :type Integer))
  (returns (FoundTile :type "/Game/Blueprints/BP_Tile Object Reference") (OutputPin :type "/Game/Blueprints/BP_Tile Object Reference"))
  (for _array_element (`self.Tiles`)
    _))

(fn `GridToWorld`
  (params (GridX :type Integer) (GridY :type Integer))
  (returns (WorldLocation :type "Vector Structure")))

(fn `UserConstructionScript`)