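; BP_Unit is a clickable unit that occupies a cell on a tile grid managed by BP_BoardManager.
; Clicking toggles selection and, when selected, registers the unit as the board manager's SelectedUnit; unselecting leaves that reference untouched.
; ExecuteMove passes the target coordinates to MoveToGrid, which stores them and teleports the unit to the tile's location, indexing Tiles with a hard-coded stride of seven.
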(event `self.ReceiveActorOnClicked`
  (params (ButtonPressed :type "Key Structure"))
  (set `self.IsSelected` (not (`self.IsSelected`)))
  (if (`self.IsSelected`)
    (`self.SelectUnit`)
    (`KismetSystemLibrary.PrintString` "SELECTED")
    (else
      (`KismetSystemLibrary.PrintString` "UNSELECTED"))))

(fn `ExecuteMove`
  (`self.MoveToGrid` (`self.TargetGridX`) (`self.TargetGridY`)))

(fn `MoveToGrid`
  (params (NewGridX :type Integer) (NewGridY :type Integer))
  (set `self.GridX` NewGridX)
  (set `self.GridY` NewGridY)
  (bind _returnvalue (`GameplayStatics.GetActorOfClass` "/Game/BP_BoardManager.BP_BoardManager_C"))
  (`self.K2_SetActorLocation` (`self.K2_GetActorLocation` (`|GetArrayItem` (`/Game/BP_BoardManager.Tiles` _returnvalue) (+ (* (`local.NewGridX`) 7) (`local.NewGridY`))))))

(fn `SelectUnit`
  (bind _returnvalue (`GameplayStatics.GetActorOfClass` "/Game/BP_BoardManager.BP_BoardManager_C"))
  (set `/Game/BP_BoardManager.SelectedUnit` self _returnvalue)
  (`KismetSystemLibrary.PrintString` "UNIT STORED"))

(fn `UserConstructionScript`)