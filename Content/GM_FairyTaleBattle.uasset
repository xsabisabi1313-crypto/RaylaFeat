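; GM_FairyTaleBattle holds the rules for an elemental unit battle, apparently as the game mode.
; CHeckElementAdvantage applies a Fire > Grass > Water > Fire triangle.
; BattleUnits uses it to double an advantaged unit's power, then compares both and returns a Japanese win or draw string.
; DamageBase is unfinished: its player branch is empty and the PlayerBaseHP subtraction is unwired; BeginPlay and Tick are empty.
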(fn `BattleUnits`
  (params (Unit1_Power :type Integer) (Unit1_Element :type "/Game/E_Element Enum" :default "NewEnumerator0") (Unit2_Power :type Integer) (Unit2_Element :type "/Game/E_Element Enum" :default "NewEnumerator0"))
  (returns (Result :type String))
  (locals (Final_Unit1_Power :type Integer) (Final_Unit2_Power :type Integer))
  (bind _final_unit1_power (`local.Final_Unit1_Power`))
  (bind _final_unit2_power (`local.Final_Unit2_Power`))
  (bind _isadvantage (`self.CHeckElementAdvantage` Unit1_Element Unit2_Element))
  (if _isadvantage
    (set `local.Final_Unit1_Power` (* Unit1_Power 2))
    (else
      (set `local.Final_Unit1_Power` Unit1_Power)))
  (bind _isadvantage_2 (`self.CHeckElementAdvantage` Unit2_Element Unit1_Element))
  (if _isadvantage_2
    (set `local.Final_Unit2_Power` (* Unit2_Power 2))
    (else
      (set `local.Final_Unit2_Power` Unit2_Power)))
  (if (> _final_unit1_power _final_unit2_power)
    (return "Unit1の勝利")
    (elif (< _final_unit1_power _final_unit2_power)
      (return "Unit2の勝利")
      (else
        (return "相打ち")))))

(fn `CHeckElementAdvantage`
  (params (AttackerElement :type "/Game/E_Element Enum" :default "NewEnumerator0") (DefenderElement :type "/Game/E_Element Enum" :default "NewEnumerator0"))
  (returns (IsAdvantage :type Boolean))
  (switch `/Game/E_Element` AttackerElement
    (:`NewEnumerator0`
      (return (`|EnumEquality` DefenderElement "NewEnumerator2")))
    (:`NewEnumerator1`
      (return (`|EnumEquality` DefenderElement "NewEnumerator0")))
    (:`NewEnumerator2`
      (return (`|EnumEquality` DefenderElement "NewEnumerator1")))))

(fn `DamageBase`
  (params (IsPlayer :type Boolean) (DamageAmount :type Integer))
  (if IsPlayer
    _))

(fn `UserConstructionScript`)