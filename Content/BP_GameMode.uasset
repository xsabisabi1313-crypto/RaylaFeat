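; Game mode for a two-player, grid-based card battler, running a Spawn, Move Reserve and Battle phase loop through ChangePhase.
; Spawn grants cost, shows confirm and cost widgets, and lets SummonUnit place units on tiles.
; Move Reserve executes only Player 1's reserved move from BP_BoardManager, then Battle resolves pairs using power and a Fire/Water/Grass advantage check, destroying losers.
; Game Over is an empty stub, and DebugSpawnEnemy places a test enemy.
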(event `self.ReceiveBeginPlay`
  (`self.ChangePhase` "NewEnumerator0"))

(fn `BattleUnits`
  (params (Unit1Power :type Integer) (Unit1Element :type "/Game/E_Element Enum" :default "NewEnumerator0") (Unit2Power :type Integer) (Unit2Element :type "/Game/E_Element Enum" :default "NewEnumerator0"))
  (returns (Result :type String))
  (locals (Final_Unit1_Power :type Integer) (Final_Unit2_Power :type Integer))
  (bind _final_unit1_power (`local.Final_Unit1_Power`))
  (bind _final_unit2_power (`local.Final_Unit2_Power`))
  (bind _isadvantage (`self.CheckElementAdvantage` Unit1Element Unit2Element))
  (if _isadvantage
    (set `local.Final_Unit1_Power` (* Unit1Power 2))
    (else
      (set `local.Final_Unit2_Power` Unit2Power)))
  (bind _isadvantage_2 (`self.CheckElementAdvantage` Unit1Element Unit2Element))
  (if _isadvantage_2
    (set `local.Final_Unit2_Power` (* Unit2Power 2))
    (else
      (set `local.Final_Unit2_Power` Unit2Power)))
  (if (< _final_unit1_power _final_unit2_power)
    (return "Unit1の勝利")
    (elif (> _final_unit1_power _final_unit2_power)
      (return "Unit2の勝利")
      (else
        (return "相打ち")))))

(fn `ChangePhase`
  (params (NewPhase :type "/Game/EGamePhase Enum" :default "NewEnumerator0"))
  (`KismetSystemLibrary.PrintString` (`|GetEnumeratorNameAsString` NewPhase) true true (struct :`A` 1.0))
  (set `self.CurrentPhase` NewPhase)
  (`KismetSystemLibrary.PrintString` (`KismetStringLibrary.Conv_IntToString` (`self.TurnCount`)) true true (struct :`R` 0.018224 :`G` 0.923333 :`A` 1.0) 10.0)
  (`self.OnPhaseChanged` NewPhase)
  (switch `/Game/EGamePhase` NewPhase
    (:`NewEnumerator0`
      (bind _returnvalue (`GameplayStatics.GetActorOfClass` "/Game/BP_BoardManager.BP_BoardManager_C"))
      (set `/Game/BP_BoardManager.P1HasReserved` false _returnvalue)
      (set `/Game/BP_BoardManager.P2HasReserved` false _returnvalue)
      (`self.StartCardPhase`))
    (:`NewEnumerator1`
      (`self.StartProcess`))
    (:`NewEnumerator2`
      (`self.StartBattle`))
    (:`NewEnumerator3`
      (`self.StartGameOver`))))

(fn `CheckElementAdvantage`
  (params (AtackerElement :type "/Game/E_Element Enum" :default "NewEnumerator0") (DefenderElement :type "/Game/E_Element Enum" :default "NewEnumerator0"))
  (returns (IsAdvantage :type Boolean))
  (switch `/Game/E_Element` AtackerElement
    (:`NewEnumerator0`
      (return (`|EnumEquality` DefenderElement "NewEnumerator2")))
    (:`NewEnumerator1`
      (return (`|EnumEquality` DefenderElement "NewEnumerator0")))
    (:`NewEnumerator2`
      (return (`|EnumEquality` DefenderElement "NewEnumerator1")))))

(fn `DebugSpawnEnemy`
  (bind _returnvalue (`GameplayStatics.GetActorOfClass` "/Game/BP_BoardManager.BP_BoardManager_C"))
  (bind _foundtile (`/Game/BP_BoardManager.GetTileAt` _returnvalue 1 3))
  (bind _returnvalue_2 (`|SpawnActorFromClass` "/Game/BP_Unit_RedRidingHood.BP_Unit_RedRidingHood_C" (`self.GetTransform` _foundtile) "Undefined" "MultiplyWithRoot" null null))
  (bind _asbp_unit (cast `/Game/BP_Unit` _returnvalue_2))
  (set `/Game/BP_Unit.RowName` "RedRidingHood" _asbp_unit)
  (set `/Game/BP_Unit.OwnerPlayer` 2 _asbp_unit)
  (set `BP_UnitBase.GridX` 1 _asbp_unit)
  (set `BP_UnitBase.GridY` 3 _asbp_unit)
  (`/Game/BP_Unit.InitializeCardData` _asbp_unit))

(fn `EndCardPhase`
  (`self.ChangePhase` "NewEnumerator1"))

(fn `PlayerConfirm`
  (params (PlayerID :type Integer))
  (if (== PlayerID 1)
    (set `self.Player1Confirmed` true)))

(fn `SetSelectedUnit`
  (params (UnitReference :type "/Game/BP_Unit Object Reference"))
  (bind _returnvalue (`GameplayStatics.GetActorOfClass` "/Game/BP_BoardManager.BP_BoardManager_C"))
  (set `/Game/BP_BoardManager.P1_SelectedUnit` UnitReference _returnvalue)
  (`KismetSystemLibrary.PrintString` "UNITSTORED"))

(fn `StartBattle`
  (locals (P1MovedUnit :type "/Game/BP_Unit Object Reference") (P2MovedUnit :type "/Game/BP_Unit Object Reference"))
  (`KismetSystemLibrary.PrintString` "バトルフェーズ開始" true true (struct :`R` 0.723333 :`G` 0.214145 :`A` 1.0))
  (bind _returnvalue (`GameplayStatics.GetActorOfClass` "/Game/BP_BoardManager.BP_BoardManager_C"))
  (if (`/Game/BP_BoardManager.P1HasReserved` _returnvalue)
    (set `local.P1MovedUnit` (`/Game/BP_BoardManager.P1_SelectedUnit` _returnvalue)))
  (if (`/Game/BP_BoardManager.P2HasReserved` _returnvalue)
    (set `local.P2MovedUnit` (`/Game/BP_BoardManager.P2_SelectedUnit` _returnvalue)))
  (bind _outactors (`GameplayStatics.GetAllActorsOfClass` "/Game/BP_Unit.BP_Unit_C"))
  (bind _returnvalue_2 (`self.DetermineBattlePairs` (`local.P1MovedUnit`) (`local.P2MovedUnit`) _outactors))
  (for _array_element _returnvalue_2
    (bind _asbp_unit (cast `/Game/BP_Unit` (break `BattlePair` _array_element)))
    (bind _asbp_unit_2 (cast `/Game/BP_Unit` (`.UnitB` (break `BattlePair` _array_element))))
    (bind _result (`self.BattleUnits` (`/Game/BP_Unit.Power` _asbp_unit) (`/Game/BP_Unit.Element` _asbp_unit) (`/Game/BP_Unit.Power` _asbp_unit_2) (`/Game/BP_Unit.Element` _asbp_unit_2)))
    (switch `string` _result
      (:`Unit1の勝利`
        (`self.K2_DestroyActor` (`.UnitB` (break `BattlePair` _array_element)))
        (`KismetSystemLibrary.PrintString` "Unit1の勝利"))
      (:`Unit2の勝利`
        (`self.K2_DestroyActor` (break `BattlePair` _array_element))
        (`KismetSystemLibrary.PrintString` "Unit2の勝利"))
      (:`相打ち`
        (`self.K2_DestroyActor` (break `BattlePair` _array_element))
        (`self.K2_DestroyActor` (`.UnitB` (break `BattlePair` _array_element)))
        (`KismetSystemLibrary.PrintString` "相打ち")))
    (`KismetSystemLibrary.PrintString` "Battleフェーズ終了" true true (struct :`R` 0.776667 :`G` 0.43432 :`A` 1.0) 10.0)
    (`self.ChangePhase` "NewEnumerator0"))
  (`self.ChangePhase` "NewEnumerator0"))

(fn `StartCardPhase`
  (bind _returnvalue (`GameplayStatics.GetPlayerController` 0))
  (bind _returnvalue_2 (`GameplayStatics.GetPlayerController` 0))
  (`KismetSystemLibrary.PrintString` "cardPhaseを開始します" true true (struct :`R` 0.868268 :`B` 0.963333 :`A` 1.0) 10.0)
  (if (not (== (`self.TurnCount`) 1))
    (set `self.Player1Cost` (+ (`self.Player1Cost`) 2))
    (set `self.Player2Cost` (+ (`self.Player2Cost`) 2)))
  (bind _returnvalue_3 (`|CreateWidget` "/Game/WB_ConfirmButton.WB_ConfirmButton_C" _returnvalue))
  (`UserWidget.AddToViewport` _returnvalue_3 0)
  (bind _returnvalue_4 (`|CreateWidget` "/Game/WB_CostDisplay.WB_CostDisplay_C" _returnvalue))
  (bind _output_get (set `self.CostDisplayWidget` _returnvalue_4))
  (`UserWidget.AddToViewport` _output_get 0)
  (`/Game/WB_CostDisplay.UpdateCostDisplay` _output_get (`self.Player1Cost`) (`self.Player2Cost`))
  (`KismetSystemLibrary.PrintString` "ここから先を調整しようと思います")
  (`WidgetBlueprintLibrary.SetInputMode_GameAndUIEx` _returnvalue_2 (stale _aswb_confirm_button))
  (bind _aswb_confirm_button (cast `/Game/WB_ConfirmButton` _returnvalue_3))
  (bind _output_get_2 (set `PlayerController.bShowMouseCursor` true _returnvalue_2))
  (set `PlayerController.bEnableClickEvents` _output_get_2 _returnvalue_2))

(fn `StartGameOver`)

(fn `StartProcess`
  (`KismetSystemLibrary.PrintString` "StartProccessCalled")
  (bind _returnvalue (`GameplayStatics.GetActorOfClass` "/Game/BP_BoardManager.BP_BoardManager_C"))
  (bind _p1_selectedunit (`/Game/BP_BoardManager.P1_SelectedUnit` _returnvalue))
  (`/Engine/EditorBlueprintResources/StandardMacros.IsValid` _p1_selectedunit
    (:`Is Valid`
      (if (`/Game/BP_BoardManager.P1HasReserved` _returnvalue)
        (`/Game/BP_Unit.ExecuteMove` _p1_selectedunit (`/Game/BP_BoardManager.P1_TargetGridX` _returnvalue) (`/Game/BP_BoardManager.P1_TargetGridY` _returnvalue))
        (`self.ChangePhase` "NewEnumerator2")
        (else
          (`KismetSystemLibrary.PrintString` "プロセスフェーズを無効にしましｔ"))))))

(fn `SummonUnit`
  (params (SpawnTile :type "/Game/BP_Tile Object Reference") (UnitClass :type "/Game/BP_Unit Class Reference") (PlayerID :type Integer) (RowName :type Name))
  (bind _returnvalue (`self.GetTransform` SpawnTile))
  (bind (_isselected _targetgridx _targetgridy _power _element _rowname _ownerplayer _moverange _atackrange _atackpattern _cost) (defaults `Object` UnitClass))
  (if (`|EnumEquality` (`self.CurrentPhase`) "NewEnumerator0")
    (if (== PlayerID 1)
      (if (>= (`self.Player1Cost`) _cost)
        (bind _returnvalue_2 (`|SpawnActorFromClass` UnitClass _returnvalue "Undefined" "MultiplyWithRoot" null null))
        (set `/Game/BP_Unit.OwnerPlayer` 1 _returnvalue_2)
        (set `/Game/BP_Unit.GridX` (`/Game/BP_Tile.GridX` SpawnTile) _returnvalue_2)
        (set `/Game/BP_Unit.GridY` (`/Game/BP_Tile.GridY` SpawnTile) _returnvalue_2)
        (set `self.Player1Cost` (- (`self.Player1Cost`) (`/Game/BP_Unit.Cost` _returnvalue_2)))
        (set `self.UnitToSummon` null)
        (set `/Game/BP_Unit.RowName` RowName _returnvalue_2)
        (`/Game/BP_Unit.InitializeCardData` _returnvalue_2)
        (`KismetSystemLibrary.PrintString` "スポーンしたよ"))
      (elif (>= (`self.Player2Cost`) _cost)
        (bind _returnvalue_3 (`|SpawnActorFromClass` UnitClass _returnvalue "Undefined" "MultiplyWithRoot" null null))
        (set `/Game/BP_Unit.OwnerPlayer` 2 _returnvalue_3)
        (set `/Game/BP_Unit.GridX` (`/Game/BP_Tile.GridX` SpawnTile) _returnvalue_3)
        (set `/Game/BP_Unit.GridY` (`/Game/BP_Tile.GridY` SpawnTile) _returnvalue_3)
        (set `self.Player2Cost` (- (`self.Player2Cost`) (`/Game/BP_Unit.Cost` _returnvalue_3)))
        (set `self.UnitToSummon` null)))))

(fn `UserConstructionScript`)