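; BP_Tile is a clickable grid board tile that turns player clicks into summon or move orders, depending on the game phase.
; On click it either has BP_GameMode summon the chosen unit on itself or has BP_BoardManager reserve a move of P1SelectedUnit to its grid coordinates.
; Move and attack range functions apply the same highlight material, and ResetTile restores the normal one.
; The coordinate label update is unconnected and never runs.
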(event `self.ReceiveActorOnClicked`
  (params (ButtonPressed :type "Key Structure"))
  (`KismetSystemLibrary.PrintString` "タイルがクリックされたよ")
  (bind _asbp_game_mode (cast `/Game/BP_GameMode` (`GameplayStatics.GetGameMode`)))
  (if (`|EnumEquality` (`/Game/BP_GameMode.CurrentPhase` _asbp_game_mode) "NewEnumerator0")
    (bind _unittosummon (`/Game/BP_GameMode.UnitToSummon` _asbp_game_mode))
    (if (`KismetSystemLibrary.IsValidClass` _unittosummon)
      (`/Game/BP_GameMode.SummonUnit` _asbp_game_mode self _unittosummon (`/Game/BP_GameMode.CurrentPlayerTurn` _asbp_game_mode) (`/Game/BP_GameMode.SelectedRowName` _asbp_game_mode)))
    (elif (`|EnumEquality` (`/Game/BP_GameMode.CurrentPhase` _asbp_game_mode) "NewEnumerator1")
      (bind _returnvalue (`GameplayStatics.GetActorOfClass` "/Game/BP_BoardManager.BP_BoardManager_C"))
      (bind _asbp_unit (cast `/Game/BP_Unit` (`/Game/BP_BoardManager.P1_SelectedUnit` _returnvalue)))
      (bind _returnvalue_2 (`GameplayStatics.GetActorOfClass` "/Game/BP_BoardManager.BP_BoardManager_C"))
      (`/Game/BP_BoardManager.ReserveMove` _returnvalue_2 _asbp_unit (`self.GridX`) (`self.GridY`)))))

(fn `ResetTile`
  (`PrimitiveComponent.SetMaterial` (`self.TileMesh`) 0 (`self.NormalMaterial`)))

(fn `ShowAtackRange`
  (`PrimitiveComponent.SetMaterial` (`self.TileMesh`) 0 (`self.HighLightMaterial`)))

(fn `ShowMoveRange`
  (`PrimitiveComponent.SetMaterial` (`self.TileMesh`) 0 (`self.HighLightMaterial`)))

(fn `UserConstructionScript`)